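; BP_Boo is a Boo-style enemy actor that creeps toward the player whenever it has not been rendered recently.
; Tick checks WasRecentlyRendered; while unseen, it interpolates its location slowly toward player pawn 0 and prints a debug message.
; The same unseen branch plays the Mesh timeline, whose track drives the Translucency material parameter on the static mesh.
; BeginPlay creates and stores a dynamic instance of Booface_Mat for that mesh.
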(event EventTick
  (params (DeltaSeconds :type Float%20%28single-precision%29))
  ;[1 1 1] Boo
  (if (not (Class|Actor|WasRecentlyRendered 0.1))
    (Utilities|FlowControl|Sequence
      (:then_0
        (Development|PrintString "Boo is coming..." true true "(R=0.000000,G=0.660000,B=1.000000,A=1.000000)" 0.5 "1")
        (Transformation|SetActorLocationAndRotation (Math|Interpolation|VInterpTo (Transformation|GetActorLocation) (Transformation|GetActorLocation (Game|Player|GetPlayerPawn 0)) DeltaSeconds 0.5) "0, 0, 0"))
      (:then_1
        (bind _newtrack_0 (Timeline|Mesh Play)
          (:Update
            (bind _output_get (Variables|Default|Setblend%20value _newtrack_0))
            (Rendering|Material|SetScalarParameterValueonMaterials (Variables|Default|GetStatic%20Mesh) "Translucency" _output_get)))))))

(event EventBeginPlay
  ;[1 1 1] Boo
  (bind _returnvalue (Rendering|Material|CreateDynamicMaterialInstance (Variables|Default|GetStatic%20Mesh) 0 "/Game/MAterials/booface_Mat.booface_Mat" "None" :!class /Script/Engine.PrimitiveComponent))
  (Variables|Default|SetBlend%20Instance%20Dynamic _returnvalue))

(fn ConstructionScript)