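; Player character that looks around with the mouse and moves by point-and-click teleporting, likely a gaze-interaction prototype.
; Each tick, a camera line trace stores any interface-implementing hit actor as InteractingActor and records the hit point at a fixed height.
; Left click teleports there when no such actor is targeted and the surface is not too steep.
; Strafe input is unwired, and the Move_To and Teleport graphs are empty.
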(event Custom|GazeCheck
  (bind _camera (Variables|Default|GetCamera))
  (bind _returnvalue (Transformation|GetWorldLocation _camera))
  ;[1 1 1] Gaze check
  (bind _outhit (Collision|LineTraceByChannel _returnvalue (+ _returnvalue (* (Math|Vector|GetForwardVector _camera) 2000)) "TraceTypeQuery1" false 0 "ForOneFrame"))
  (Utilities|FlowControl|Sequence
    (:then_0
      (if (Utilities|DoesObjectImplementInterface (.HitActor (Collision|BreakHitResult _outhit)) 0)
        (Variables|Default|SetinteractingActor (.HitActor (Collision|BreakHitResult _outhit)))
        (else
          (Variables|Default|SetinteractingActor 0))))
    (:then_1
      (Class|KismetMathLibrary|VectorSet (Variables|Default|GetTraceLoc) (.X (Math|Vector|BreakVector (.Location (Collision|BreakHitResult _outhit)))) (.Y (Math|Vector|BreakVector (.Location (Collision|BreakHitResult _outhit)))) 112.0))))

(event EventTick
  (params (DeltaSeconds :type Float%20%28single-precision%29))
  ;[1 1 1] Gaze check
  (CallFunction|GazeCheck))

(event Input|AxisEvents|InputAxismouseX
  (params (AxisValue :type Float%20%28single-precision%29))
  ;[1 1 1] Input
  (Pawn|Input|AddControllerYawInput AxisValue))

(event Input|AxisEvents|InputAxismouseY
  (params (AxisValue :type Float%20%28single-precision%29))
  ;[1 1 1] Input
  (Pawn|Input|AddControllerPitchInput AxisValue))

(event Input|MouseEvents|LeftMouseButton
  (params (Key :type Key%20Structure :default "None"))
  ;[1 1 1] Gaze check
  (:Pressed
    (Utilities|IsValid (Variables|Default|GetinteractingActor)
      (:Is%20Not%20Valid
        (if (>= (.Z (Math|Vector|BreakVector (.Normal (Collision|BreakHitResult (stale Custom|GazeCheck _outhit))))) 0.2)
          (Transformation|Teleport (Variables|Default|GetTraceLoc) (Transformation|GetActorRotation)))))))

(fn ConstructionScript)

(fn Moveto)

(fn Teleport)